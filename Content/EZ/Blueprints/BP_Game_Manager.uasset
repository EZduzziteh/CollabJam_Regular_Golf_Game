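; Level manager for the golf shooter that tracks enemies, detects victory and handles saving and level transitions.
; BeginPlay equips the revolver if unlocked and loads the save object, whose per-type kill counters increase as enemies are removed.
; Enemy list changes fire a dispatcher; an empty list after the invasion triggers a win.
; Winning clears projectiles, enemies and music, plays a victory sound, async-saves, then opens the next level; EndGame saves and opens the end menu.
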(event `End Game`
  ; end game
  (`AsyncActionHandleSaveGame.AsyncSaveGameToSlot` (`self.Save Game Data`) (`self.SaveSlotName`)
    (:`Completed`
      (`GameplayStatics.OpenLevelBySoftObjectPtr` "/Game/_Maps/_Menu_End._Menu_End"))))

(event `self.ReceiveBeginPlay`
  (`|ExecutionSequence`
    (:`then_0`
      (add `self.OnEnemiesChanged` (delegate `CheckEnemies`))
      (if (`self.UnlockedRevolver`)
        (bind _asbp_golf_shooter_character (cast `/Game/EZ/Blueprints/Player_Character/BP_Golf_Shooter_Character` (`GameplayStatics.GetPlayerPawn` 0)))
        (set `/Game/EZ/Blueprints/Player_Character/BP_Golf_Shooter_Character.Primary Weapon` "/Game/EZ/Blueprints/WeaponSystem/DataAssets/Weapon_Revolver.Weapon_Revolver" _asbp_golf_shooter_character)
        (`/Game/EZ/Blueprints/Player_Character/BP_Golf_Shooter_Character.Initialize Animations` _asbp_golf_shooter_character)))
    (:`then_1`
      (bind _returnvalue (`GameplayStatics.LoadGameFromSlot` (`self.SaveSlotName`)))
      (`/Engine/EditorBlueprintResources/StandardMacros.IsValid` _returnvalue
        (:`Is Valid`
          (bind _asbp_golf_shooter_save_game (cast `/Game/EZ/Blueprints/BP_GolfShooter_SaveGame` _returnvalue))
          (set `self.Save Game Data` _asbp_golf_shooter_save_game))
        (:`Is Not Valid`
          (`KismetSystemLibrary.PrintString` "save slot not initialized"))))))

(event `CheckEnemies`
  ; Check Win condition
  (if (`self.IsInvasionTriggered`)
    (if (<= (`KismetArrayLibrary.Array_Length` (`self.Enemies`)) 0)
      (`self.WinLevel`))))

(event `WinLevel`
  ; Win Level
  (if (`self.Winning`)
    (`KismetSystemLibrary.PrintString` "already winning")
    (else
      (set `self.Winning` true)
      (`self.StopGamePlayForWin`)
      (bind _returnvalue (`GameplayStatics.GetActorOfClass` "/Game/EZ/Blueprints/BP_MusicManager.BP_MusicManager_C"))
      (`self.K2_DestroyActor` _returnvalue)
      (`KismetSystemLibrary.PrintString` "Win Level")
      (`GameplayStatics.PlaySound2D` (`self.Victory Sound Effect`) 0.6 1.0 0.0 null null)
      ;; Load Next Level
      (`AsyncActionHandleSaveGame.AsyncSaveGameToSlot` (`self.Save Game Data`) (`self.SaveSlotName`)
        (:`Completed`
          (`KismetSystemLibrary.Delay` (+ 0.3 (`SoundBase.Duration` (`self.Victory Sound Effect`))))
          (`GameplayStatics.OpenLevelBySoftObjectPtr` (`self.LevelToLoad`)))))))

(event `Add Enemy`
  (params (NewItem :type "/Game/EZ/Blueprints/AI/BP_Enemy_Base Object Reference (by ref)"))
  ; Add enemy
  (`KismetArrayLibrary.Array_AddUnique` (`self.Enemies`) NewItem)
  (`self.OnEnemiesChanged`))

(event `Remove Enemy`
  (params (Item :type "/Game/EZ/Blueprints/AI/BP_Enemy_Base Object Reference (by ref)"))
  (bind _save_game_data (`self.Save Game Data`))
  ; Remove enemy
  (`KismetSystemLibrary.PrintString` (`KismetStringLibrary.Concat_StrStr` "Removing :" (`|GetEnumeratorNameAsString` (`/Game/EZ/Blueprints/AI/BP_Enemy_Base.EnemyType` Item))))
  (`KismetArrayLibrary.Array_RemoveItem` (`self.Enemies`) Item)
  (switch `/Game/EZ/Blueprints/AI/E_EnemyType` (`/Game/EZ/Blueprints/AI/BP_Enemy_Base.EnemyType` Item)
    (:`NewEnumerator0`
      (`/Engine/EditorBlueprintResources/StandardMacros.IncrementInt` (`/Game/EZ/Blueprints/BP_GolfShooter_SaveGame.SoldierAliensKilled` _save_game_data)
        (:`  `
          _)))
    (:`NewEnumerator1`
      (`/Engine/EditorBlueprintResources/StandardMacros.IncrementInt` (`/Game/EZ/Blueprints/BP_GolfShooter_SaveGame.ShipAliensKilled` _save_game_data)
        (:`  `
          _)))
    (:`NewEnumerator2`
      (`/Engine/EditorBlueprintResources/StandardMacros.IncrementInt` (`/Game/EZ/Blueprints/BP_GolfShooter_SaveGame.SexyAliensKilled` _save_game_data)
        (:`  `
          _))))
  (`self.OnEnemiesChanged`))

(fn `StopGamePlayForWin`
  (bind _outactors (`GameplayStatics.GetAllActorsOfClass` "/Game/EZ/Blueprints/Projectiles/BP_Projectile.BP_Projectile_C"))
  (for _array_element _outactors
    (`self.K2_DestroyActor` _array_element))
  (bind _outactors_2 (`GameplayStatics.GetAllActorsOfClass` "/Game/EZ/Blueprints/AI/BP_Enemy_Base.BP_Enemy_Base_C"))
  (for _array_element_2 _outactors_2
    (`self.K2_DestroyActor` _array_element_2)))

(fn `UserConstructionScript`)