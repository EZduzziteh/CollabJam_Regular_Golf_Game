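; Health pack pickup that restores health to the GolfShooterCharacter that collects it.
; Its Handle Pickup override adds HealAmount to the character's current health, caps it at MaxHealth, then calls the parent pickup handler.
; The event graph holds only disabled default nodes, and the construction script just calls its parent.
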(fn `Handle Pickup`
  (params (`Golf Shooter Character` :type "/Game/EZ/Blueprints/BP_Golf_Shooter_Character Object Reference"))
  (bind _maxhealth (`/Game/EZ/Blueprints/BP_Golf_Shooter_Character.maxHealth` `Golf Shooter Character`))
  (bind _output_get (set `/Game/EZ/Blueprints/BP_Golf_Shooter_Character.currentHealth` (+ (`/Game/EZ/Blueprints/BP_Golf_Shooter_Character.currentHealth` `Golf Shooter Character`) (`self.Heal Amount`)) `Golf Shooter Character`))
  (if (>= _output_get _maxhealth)
    (set `/Game/EZ/Blueprints/BP_Golf_Shooter_Character.currentHealth` _maxhealth `Golf Shooter Character`))
  (`parent.Handle Pickup` `Golf Shooter Character`))

(fn `UserConstructionScript`
  (`parent.UserConstructionScript`))