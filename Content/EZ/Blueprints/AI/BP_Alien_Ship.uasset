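; Alien ship pawn that provides movement, aiming and burst-fire actions, with no decision logic of its own.
; MoveTowardsLocation adds movement input toward a target, and LookAtLocation snaps the actor's rotation to face one.
; ProjectileBurst starts a self-calling, delay-spaced SpawnProjectile loop that fires from the spawn point with random pitch-varied laser sounds, yielding one shot more than the requested count.
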(event `Projectile Burst`
  (params (`Burst Count` :type Integer))
  (set `self.currentBurstCount` `Burst Count`)
  (`self.Spawn Projectile`))

(event `Spawn Projectile`
  (bind _projectile_spawn_point (`self.Projectile Spawn Point`))
  (bind _returnvalue (`SceneComponent.K2_GetComponentLocation` _projectile_spawn_point))
  (`GameplayStatics.PlaySoundAtLocation` (`KismetArrayLibrary.Array_Random` (`self.Laser Sounds`)) _returnvalue (struct) 1.0 (`KismetMathLibrary.RandomFloatInRange` 0.8 1.2) 0.0 null null null null)
  (`|SpawnActorFromClass` (`self.Projectile`) (`KismetMathLibrary.MakeTransform` _returnvalue (`SceneComponent.K2_GetComponentRotation` _projectile_spawn_point)) "AlwaysSpawn" "MultiplyWithRoot" null null)
  (`KismetSystemLibrary.Delay` (`self.Burst Delay`))
  (if (> (`self.currentBurstCount`) 0)
    (`self.Spawn Projectile`)
    (`/Engine/EditorBlueprintResources/StandardMacros.DecrementInt` (`self.currentBurstCount`))))

(fn `LookAtLocation`
  (params (Location :type "Vector Structure"))
  (`self.K2_SetActorRotation` (`KismetMathLibrary.FindLookAtRotation` (`self.K2_GetActorLocation`) Location)))

(fn `MoveTowardsLocation`
  (params (targetLocation :type "Vector Structure") (DeltaTime :type "Float (double-precision)"))
  (`self.AddMovementInput` (- (`local.targetLocation`) (`self.K2_GetActorLocation`))))

(fn `UserConstructionScript`)