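; AI controller for the alien soldier that hunts and shoots golf shooter characters.
; On possess it starts looping timers for target search and firing.
; The search takes the first character from a sphere overlap and drops it beyond lose-sight range.
; Tick turns the soldier toward its target and moves it to an offset position until within acceptance range, while the fire timer spawns projectiles within shooting range.
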(event `self.ReceiveTick`
  (params (DeltaSeconds :type "Float (single-precision)"))
  (`/Engine/EditorBlueprintResources/StandardMacros.IsValid` (`self.Current Target`)
    (:`Is Valid`
      (`/Game/EZ/Blueprints/AI/BP_Alien_Soldier.LookAtLocation` (`self.Alien Soldier Reference`) (`self.K2_GetActorLocation` (`self.Current Target`)))
      (if (not (< (`KismetMathLibrary.Vector_Distance` (`self.K2_GetActorLocation` (`self.Current Target`)) (`self.K2_GetActorLocation` (`self.Alien Soldier Reference`))) (`self.Movement Acceptance Range`)))
        (`/Game/EZ/Blueprints/AI/BP_Alien_Soldier.MoveTowardsLocation` (`self.Alien Soldier Reference`) (+ (`self.DesiredTargetOffset`) (`self.K2_GetActorLocation` (`self.Current Target`))) 0.0)))))

(event `self.ReceivePossess`
  (params (PossessedPawn :type "Pawn Object Reference"))
  (bind _asbp_alien_soldier (cast `/Game/EZ/Blueprints/AI/BP_Alien_Soldier` PossessedPawn)
    (:`then`
      (set `self.Alien Soldier Reference` _asbp_alien_soldier)
      (`KismetSystemLibrary.K2_SetTimerDelegate` (delegate `Search For Target`) 2.0 true true)
      (`KismetSystemLibrary.K2_SetTimerDelegate` (delegate `Try Fire`) 2.0 true true))
    (:`CastFailed`
      (`KismetSystemLibrary.PrintString` "no alien soldiear"))))

(event `self.ReceiveBeginPlay`)

(event `Try Fire`
  (`/Engine/EditorBlueprintResources/StandardMacros.IsValid` (`self.Current Target`)
    (:`Is Valid`
      (if (< (`KismetMathLibrary.Vector_Distance` (`self.K2_GetActorLocation` (`self.Current Target`)) (`self.K2_GetActorLocation` (`self.Alien Soldier Reference`))) (`self.Shooting Range`))
        (`/Game/EZ/Blueprints/AI/BP_Alien_Soldier.Spawn Projectile` (`self.Alien Soldier Reference`))))))

(event `Search For Target`
  (bind _detection_range (`self.Detection Range`))
  (bind _returnvalue (`self.K2_GetActorLocation` (`self.K2_GetPawn`)))
  ; Search For Target
  (`/Engine/EditorBlueprintResources/StandardMacros.IsValid` (`self.Current Target`)
    (:`Is Valid`
      ; Lose Target
      (if (> (`KismetMathLibrary.Vector_Distance` (`self.K2_GetActorLocation` (`self.Current Target`)) _returnvalue) (`self.LoseSightRange`))
        (set `self.Current Target` null)))
    (:`Is Not Valid`
      (if (`self.Debug`)
        (`KismetSystemLibrary.PrintString` "Searching for target")
        (`KismetSystemLibrary.DrawDebugSphere` _returnvalue _detection_range 12 (struct :`R` 1.0 :`G` 0.409537 :`B` 0.952164 :`A` 1.0) 3.0 0.5))
      (bind _outactors (`KismetSystemLibrary.SphereOverlapActors` _returnvalue _detection_range (`|MakeArray` "ObjectTypeQuery9" :!type "EObjectTypeQuery Enum") "/Game/EZ/Blueprints/Player_Character/BP_Golf_Shooter_Character.BP_Golf_Shooter_Character_C"))
      (for _array_element _outactors
        (set `self.Current Target` _array_element)
        (break))
      (`KismetSystemLibrary.PrintString` "No target found!"))))

(fn `UserConstructionScript`)