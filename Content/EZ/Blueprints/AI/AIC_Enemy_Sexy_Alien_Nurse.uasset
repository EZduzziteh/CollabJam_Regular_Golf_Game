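; AI controller for the Alien Nurse enemy that overrides the parent's Attack with a knockback hit on the player.
; Attack checks that the current target is valid and inside the pawn's AttackRange, then casts it to the golf shooter character.
; It applies fixed damage and a velocity-change impulse away from the enemy with some upward lift.
; The parent Attack is never called, and a debug string prints on each in-range attack.
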(fn `Attack`
  (`/Engine/EditorBlueprintResources/StandardMacros.IsValid` (`self.Current Target`)
    (:`Is Valid`
      (if (< (`KismetMathLibrary.Vector_Distance` (`self.K2_GetActorLocation` (`self.Current Target`)) (`self.K2_GetActorLocation` (`self.Enemy Pawn Reference`))) (`/Game/EZ/Blueprints/AI/BP_Enemy_Base.AttackRange` (`self.Enemy Pawn Reference`)))
        (`KismetSystemLibrary.PrintString` "Attack!")
        (bind _asbp_golf_shooter_character (cast `/Game/EZ/Blueprints/Player_Character/BP_Golf_Shooter_Character` (`self.Current Target`)))
        (bind _returnvalue (`self.K2_GetActorLocation` _asbp_golf_shooter_character))
        (`/Game/EZ/Blueprints/Player_Character/BP_Golf_Shooter_Character.TakeDamage` _asbp_golf_shooter_character 20 _returnvalue (0.0 0.0 0.0))
        ; Apply Knockback
        (`CharacterMovementComponent.AddImpulse` (`Character.CharacterMovement` _asbp_golf_shooter_character) (+ (* (`KismetMathLibrary.Normal` (- _returnvalue (`self.K2_GetActorLocation` (`self.Enemy Pawn Reference`)))) 2000.0) (* (`KismetMathLibrary.Vector_Up`) 300.0)) true)))))

(fn `UserConstructionScript`
  (`parent.UserConstructionScript`))