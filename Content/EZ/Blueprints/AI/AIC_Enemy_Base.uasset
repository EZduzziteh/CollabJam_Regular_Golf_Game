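; Base AI controller for BP_Enemy_Base pawns that hunts the golf shooter player and fires projectile bursts.
; Staggered looping timers acquire targets by sphere overlap, drop them by distance and attack within range, registering the enemy as the player's combatant.
; Tick drives the pawn directly: closing to desired range, facing the player's camera and grounding it.
; Damage without a target massively inflates detection range, so the next search finds the player.
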(event `self.ReceiveTick`
  (params (DeltaSeconds :type "Float (single-precision)"))
  ; Tick
  (`|ExecutionSequence`
    (:`then_0`
      (`/Engine/EditorBlueprintResources/StandardMacros.IsValid` (`self.Current Target`)
        (:`Is Valid`
          (`self.Determine Movement` DeltaSeconds))))
    (:`then_1`
      (`self.Face Player`))
    (:`then_2`
      (`/Game/EZ/Blueprints/AI/BP_Enemy_Base.Ground Actor` (`self.Enemy Pawn Reference`)))))

(event `self.ReceivePossess`
  (params (PossessedPawn :type "Pawn Object Reference"))
  ; On Poessess
  (bind _returnvalue (`GameplayStatics.GetActorOfClass` "/Game/EZ/Blueprints/Player_Character/BP_Golf_Shooter_Character.BP_Golf_Shooter_Character_C"))
  (bind _output_get (set `self.Player Reference` _returnvalue))
  (`/Engine/EditorBlueprintResources/StandardMacros.IsValid` _output_get
    (:`Is Valid`
      (`KismetSystemLibrary.PrintString` "Palyer valid"))
    (:`Is Not Valid`
      _))
  (`self.Set Enemy Pawn Reference` PossessedPawn)
  (`self.Target Uodate`)
  (add `/Game/EZ/Blueprints/AI/BP_Enemy_Base.OnTakeDamage` (`self.Enemy Pawn Reference`) (delegate `Handle Pawn Took Damage`))
  ;; random variation so enemies dont all check their stuff on the same frame
  (`KismetSystemLibrary.Delay` (`KismetMathLibrary.RandomFloatInRange` 0.1 0.7))
  (`KismetSystemLibrary.K2_SetTimerDelegate` (delegate `Target Uodate`) (`self.Check For Target Cooldown`) true true)
  (`KismetSystemLibrary.K2_SetTimerDelegate` (delegate `TryAttack`) (`/Game/EZ/Blueprints/AI/BP_Enemy_Base.Attack Cooldown` (`self.Enemy Pawn Reference`)) true true))

(event `Handle Pawn Took Damage`
  (params (Damager :type "Actor Object Reference"))
  ; On Poessess
  (`/Engine/EditorBlueprintResources/StandardMacros.IsValid` (`self.Current Target`)
    (:`Is Not Valid`
      ; set detection range really high (we can make this better later, shoudl ajust set target but works for now)
      (set `/Game/EZ/Blueprints/AI/BP_Enemy_Base.Detection Range` 9999999.0 (`self.Enemy Pawn Reference`)))))

(event `TryAttack`
  ; Try Fire
  (`self.Attack`))

(event `Target Uodate`
  ; Update Target
  (`/Engine/EditorBlueprintResources/StandardMacros.IsValid` (`self.Current Target`)
    (:`Is Valid`
      (`self.LoseTarget`))
    (:`Is Not Valid`
      (`self.Search For Target`))))

(fn `AIC_Enemy_Base_AutoGenFunc`
  (bind _asbp_golf_shooter_character (cast `/Game/EZ/Blueprints/Player_Character/BP_Golf_Shooter_Character` (`self.Current Target`)))
  (`/Game/EZ/Blueprints/Player_Character/BP_Golf_Shooter_Character.Remove Combatant` _asbp_golf_shooter_character (`self.Enemy Pawn Reference`)))

(fn `Attack`
  (`/Engine/EditorBlueprintResources/StandardMacros.IsValid` (`self.Current Target`)
    (:`Is Valid`
      (if (< (`KismetMathLibrary.Vector_Distance` (`self.K2_GetActorLocation` (`self.Current Target`)) (`self.K2_GetActorLocation` (`self.Enemy Pawn Reference`))) (`/Game/EZ/Blueprints/AI/BP_Enemy_Base.AttackRange` (`self.Enemy Pawn Reference`)))
        (`/Game/EZ/Blueprints/AI/BP_Enemy_Alien_Ship.Projectile Burst` (`self.Enemy Pawn Reference`) (`KismetMathLibrary.RandomIntegerInRange` 0 (`/Game/EZ/Blueprints/AI/BP_Enemy_Base.MaxBurstCount` (`self.Enemy Pawn Reference`))))))))

(fn `Determine Movement`
  (params (DeltaTime :type "Float (double-precision)"))
  ; Move Within Range to Target
  (bind _movementtarget (`self.GetMovementTarget`))
  (if (not (< (`KismetMathLibrary.Vector_Distance` (`self.K2_GetActorLocation` _movementtarget) (`self.K2_GetActorLocation` (`self.Enemy Pawn Reference`))) (`/Game/EZ/Blueprints/AI/BP_Enemy_Base.Desired Range` (`self.Enemy Pawn Reference`))))
    (`/Game/EZ/Blueprints/AI/BP_Enemy_Alien_Ship.MoveTowardsLocation` (`self.Enemy Pawn Reference`) (+ (`/Game/EZ/Blueprints/AI/BP_Enemy_Base.Desired Target Offset` (`self.Enemy Pawn Reference`)) (`self.K2_GetActorLocation` _movementtarget)) DeltaTime)))

(fn `Face Player`
  (`/Engine/EditorBlueprintResources/StandardMacros.IsValid` (`self.Player Reference`)
    (:`Is Valid`
      (`/Game/EZ/Blueprints/AI/BP_Enemy_Alien_Ship.LookAtLocation` (`self.Enemy Pawn Reference`) (`SceneComponent.K2_GetComponentLocation` (`/Game/FirstPerson/Blueprints/BP_FirstPersonCharacter.FirstPersonCamera` (`self.Player Reference`)))))
    (:`Is Not Valid`
      (`KismetSystemLibrary.PrintString` "no player")
      (bind _returnvalue (`GameplayStatics.GetActorOfClass` "/Game/EZ/Blueprints/Player_Character/BP_Golf_Shooter_Character.BP_Golf_Shooter_Character_C"))
      (set `self.Player Reference` _returnvalue))))

(fn `GetMovementTarget`
  (returns (MovementTarget :type "Actor Object Reference"))
  (return (`self.Current Target`)))

(fn `LoseTarget`
  ; Lose Target
  (if (> (`KismetMathLibrary.Vector_Distance` (`self.K2_GetActorLocation` (`self.Current Target`)) (`self.K2_GetActorLocation` (`self.Enemy Pawn Reference`))) (`/Game/EZ/Blueprints/AI/BP_Enemy_Base.LoseTargetRange` (`self.Enemy Pawn Reference`)))
    (bind _asbp_golf_shooter_character (cast `/Game/EZ/Blueprints/Player_Character/BP_Golf_Shooter_Character` (`self.Current Target`))
      (:`then`
        (`/Game/EZ/Blueprints/Player_Character/BP_Golf_Shooter_Character.Remove Combatant` _asbp_golf_shooter_character (`self.Enemy Pawn Reference`)))
      (:`CastFailed`
        _))
    (set `self.Current Target` null)))

(fn `Search For Target`
  (bind _enemy_pawn_reference (`self.Enemy Pawn Reference`))
  (bind _returnvalue (`self.K2_GetActorLocation` (`self.K2_GetPawn`)))
  (bind _detection_range (`/Game/EZ/Blueprints/AI/BP_Enemy_Base.Detection Range` (`self.Enemy Pawn Reference`)))
  ; Search For Target
  (if (`self.Debug`)
    (`KismetSystemLibrary.DrawDebugSphere` _returnvalue _detection_range 12 (struct :`R` 1.0 :`G` 0.409537 :`B` 0.952164 :`A` 1.0) 3.0 0.5))
  (bind _outactors (`KismetSystemLibrary.SphereOverlapActors` _returnvalue _detection_range (`|MakeArray` "ObjectTypeQuery9" :!type "EObjectTypeQuery Enum") "/Game/EZ/Blueprints/Player_Character/BP_Golf_Shooter_Character.BP_Golf_Shooter_Character_C"))
  (for _array_element _outactors
    (bind _output_get (set `self.Current Target` _array_element))
    (bind _asbp_golf_shooter_character (cast `/Game/EZ/Blueprints/Player_Character/BP_Golf_Shooter_Character` _output_get)
      (:`then`
        (`/Game/EZ/Blueprints/Player_Character/BP_Golf_Shooter_Character.Add Combatant` _asbp_golf_shooter_character _enemy_pawn_reference)
        (add `/Game/EZ/Blueprints/AI/BP_Enemy_Base.OnDeath` _enemy_pawn_reference (`|CreateDelegate` :!event `AIC_Enemy_Base_AutoGenFunc`))
        (break))
      (:`CastFailed`
        (break))))
  (return))

(fn `Set Enemy Pawn Reference`
  (params (Object :type "Object Object Reference"))
  (bind _asbp_enemy_base (cast `/Game/EZ/Blueprints/AI/BP_Enemy_Base` Object)
    (:`then`
      (set `self.Enemy Pawn Reference` _asbp_enemy_base))
    (:`CastFailed`
      (`KismetSystemLibrary.PrintString` "No Enemy Base!"))))

(fn `SetCurrentTarget`
  (params (NewTarget :type "Actor Object Reference"))
  (bind _output_get (set `self.Current Target` NewTarget))
  (`BlackboardComponent.SetValueAsObject` (`AIBlueprintHelperLibrary.GetBlackboard` null) "TargetActor" _output_get))

(fn `UserConstructionScript`)