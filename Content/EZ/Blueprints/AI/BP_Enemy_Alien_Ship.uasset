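; BP_Enemy_Alien_Ship is an enemy alien ship that can abduct a ball and later drop it.
; AbductBall stores the ball, turns off its mesh physics and snaps it to BallHoldPoint.
; DropHeldBall detaches the held ball, restores physics, sets CanWin on the BP_Hole actor and launches the ball via SpitOutFromMonster.
; Neither function is called within these graphs.
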(fn `AbductBall`
  (params (Ball :type "/Game/Pants/Blueprints/BP_GolfBall Object Reference"))
  (bind _output_get (set `self.HeldBall` Ball))
  (set `self.bHasBall` true)
  (`PrimitiveComponent.SetSimulatePhysics` (`/Game/Pants/Blueprints/BP_GolfBall.BallMesh` _output_get) false)
  (`self.K2_AttachToComponent` _output_get (`self.BallHoldPoint`) "None" "SnapToTarget" "KeepWorld" "KeepWorld" true))

(fn `DropHeldBall`
  (bind _heldball (`self.HeldBall`))
  (if (`self.bHasBall`)
    (`self.K2_DetachFromActor` _heldball "KeepRelative" "KeepRelative" "KeepRelative")
    (`PrimitiveComponent.SetSimulatePhysics` (`/Game/Pants/Blueprints/BP_GolfBall.BallMesh` _heldball) true)
    (bind _returnvalue (`GameplayStatics.GetActorOfClass` "/Game/EZ/Blueprints/Gameplay/BP_Hole.BP_Hole_C"))
    (set `/Game/EZ/Blueprints/Gameplay/BP_Hole.bCanWin` true _returnvalue)
    (`/Game/Pants/Blueprints/BP_GolfBall.SpitOutFromMonster` _heldball (`SceneComponent.K2_GetComponentLocation` (`self.BallHoldPoint`)) 100.0 200.0 0.25)
    (set `self.bHasBall` false)
    (set `self.HeldBall` null)))

(fn `UserConstructionScript`)