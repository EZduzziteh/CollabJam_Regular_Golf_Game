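; AI controller for the alien enemy ship, layering random dodging and ball-return behavior over its parent's movement logic.
; From possession, a looping timer with random delay picks nearby dodge points while no ball is held, accepting only those with a downward trace hit.
; An active dodge overrides parent movement until the ship nears the point.
; When carrying a ball, the movement target becomes that ball's start point.
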(event `self.ReceiveTick`
  (params (DeltaSeconds :type "Float (single-precision)"))
  (`parent.ReceiveTick` DeltaSeconds)
  (if (`self.Dodging`)
    (if (< (`KismetMathLibrary.Vector_Distance` (`self.Dodge Target`) (`self.K2_GetActorLocation` (`self.Enemy Pawn Reference`))) 25.0)
      (set `self.Dodging` false))))

(event `self.ReceivePossess`
  (params (PossessedPawn :type "Pawn Object Reference"))
  (`parent.ReceivePossess` PossessedPawn)
  (`self.TryDodge`))

(event `TryDodge`
  (`|ExecutionSequence`
    (:`then_0`
      (if (not (`self.Dodging`))
        (bind _asbp_enemy_alien_ship (cast `/Game/EZ/Blueprints/AI/BP_Enemy_Alien_Ship` (`self.Enemy Pawn Reference`))
          (:`then`
            (if (not (`/Game/EZ/Blueprints/AI/BP_Enemy_Alien_Ship.bHasBall` _asbp_enemy_alien_ship))
              (bind _output_get (set `self.Dodge Target` (+ (`self.K2_GetActorLocation`) (* (`KismetMathLibrary.RandomUnitVector`) (`KismetMathLibrary.RandomFloatInRange` 200.0 400.0)))))
              ; make sure we hit a terrain or something so we dont fly under it
              (bind (_outhit _returnvalue) (`KismetSystemLibrary.LineTraceSingle` _output_get (- _output_get (0.0 0.0 5000.0)) "TraceTypeQuery1"))
              (if _returnvalue
                (set `self.Dodging` true)
                (else
                  (set `self.Dodging` false)))))
          (:`CastFailed`
            (`KismetSystemLibrary.PrintString` "not an enemy ship!")))))
    (:`then_1`
      (`KismetSystemLibrary.Delay` (`KismetMathLibrary.RandomFloatInRange` 1.5 3.0))
      (`self.TryDodge`))))

(fn `Determine Movement`
  (params (DeltaTime :type "Float (double-precision)"))
  (if (`self.Dodging`)
    (`KismetSystemLibrary.PrintString` "try dfodge mvoe")
    (`/Game/EZ/Blueprints/AI/BP_Enemy_Base.MoveTowardsLocation` (`self.Enemy Pawn Reference`) (`self.Dodge Target`) DeltaTime)
    (else
      (`KismetSystemLibrary.PrintString` "determining movement")
      (`parent.Determine Movement` DeltaTime))))

(fn `GetMovementTarget`
  (returns (MovementTarget :type "Actor Object Reference"))
  (bind _asbp_enemy_alien_ship (cast `/Game/EZ/Blueprints/AI/BP_Enemy_Alien_Ship` (`self.Enemy Pawn Reference`))
    (:`then`
      (if (`/Game/EZ/Blueprints/AI/BP_Enemy_Alien_Ship.bHasBall` _asbp_enemy_alien_ship)
        (bind _heldball (`/Game/EZ/Blueprints/AI/BP_Enemy_Alien_Ship.HeldBall` _asbp_enemy_alien_ship))
        (`/Engine/EditorBlueprintResources/StandardMacros.IsValid` _heldball
          (:`Is Valid`
            (bind _ballstartpoint (`/Game/Pants/Blueprints/BP_GolfBall.GetBallStartPoint` _heldball))
            (`/Engine/EditorBlueprintResources/StandardMacros.IsValid` _ballstartpoint
              (:`Is Valid`
                (return _ballstartpoint))
              (:`Is Not Valid`
                _)))
          (:`Is Not Valid`
            _))))
    (:`CastFailed`
      _))
  (bind _movementtarget (`parent.GetMovementTarget`))
  (return _movementtarget))

(fn `UserConstructionScript`
  (`parent.UserConstructionScript`))