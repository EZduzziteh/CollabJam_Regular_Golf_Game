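; Alien soldier enemy that faces the player and can fire laser projectiles.
; BeginPlay runs the parent logic and caches player pawn 0, then Tick snaps the whole actor's rotation toward that pawn's location plus an offset.
; SpawnProjectile, not called within this graph, plays a random pitch-varied laser sound and spawns the projectile class at the spawn point's transform, ignoring collisions.
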(event `self.ReceiveBeginPlay`
  (`parent.ReceiveBeginPlay`)
  (set `self.PlayerReference` (`GameplayStatics.GetPlayerPawn` 0)))

(event `self.ReceiveTick`
  (params (DeltaSeconds :type "Float (single-precision)"))
  (`/Engine/EditorBlueprintResources/StandardMacros.IsValid` (`self.PlayerReference`)
    (:`Is Valid`
      (`self.K2_SetActorRotation` (`KismetMathLibrary.FindLookAtRotation` (`self.K2_GetActorLocation`) (+ (`self.K2_GetActorLocation` (`self.PlayerReference`)) (`self.Offset`)))))))

(event `Spawn Projectile`
  (bind _projectile_spawn_point (`self.Projectile Spawn Point`))
  (bind _returnvalue (`SceneComponent.K2_GetComponentLocation` _projectile_spawn_point))
  (`GameplayStatics.PlaySoundAtLocation` (`KismetArrayLibrary.Array_Random` (`self.Laser Sounds`)) _returnvalue (struct) 1.0 (`KismetMathLibrary.RandomFloatInRange` 0.8 1.2) 0.0 null null null null)
  (`|SpawnActorFromClass` (`self.Projectile Class`) (`KismetMathLibrary.MakeTransform` _returnvalue (`SceneComponent.K2_GetComponentRotation` _projectile_spawn_point)) "AlwaysSpawn" "MultiplyWithRoot" null null))

(fn `UserConstructionScript`)