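; Base enemy pawn with Paper2D flipbook visuals, providing health, damage and death effects, projectile bursts, and move and look-at helpers.
; On possession it starts the idle animation, caches the player pawn and binds a death check to its damage dispatcher.
; Bursts loop on a delay, firing BurstCount + 1 shots, each playing a shoot flipbook that reverts to idle.
; An optional per-tick downward trace snaps it to the ground.
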(event `self.ReceiveTick`
  (params (DeltaSeconds :type "Float (single-precision)"))
  ; Tick
  (if (`self.StayGrounded`)
    (`self.Ground Actor`)))

(event `Projectile Burst`
  (params (`Burst Count` :type Integer))
  ; Projectile Burst
  (set `self.currentBurstCount` `Burst Count`)
  (`self.Spawn Projectile` :!label _label)
  (`KismetSystemLibrary.Delay` (`self.Burst Delay`))
  (if (> (`self.currentBurstCount`) 0)
    (`/Engine/EditorBlueprintResources/StandardMacros.DecrementInt` (`self.currentBurstCount`)
      (:`  `
        (goto _label)))))

(event `self.ReceivePossessed`
  (params (NewController :type "Controller Object Reference"))
  ; BeginPlay
  (`self.InitializeAnimations`)
  (`self.TryGetPlayerReference`)
  (add `self.OnTakeDamage` (delegate `Check Alive`)))

(event `Check Alive`
  ; Check Alive
  (if (<= (`self.CurrentHealth`) 0)
    (`self.Die`)))

(event `/Game/EZ/Blueprints/DamageSystem/BPI_Damageable.TakeDamage`
  (params (amount :type Integer) (Location :type "Vector Structure") (Normal :type "Vector Structure"))
  ; Take Damage
  (set `self.CurrentHealth` (- (`self.CurrentHealth`) amount))
  (`GameplayStatics.PlaySoundAtLocation` (`KismetArrayLibrary.Array_Random` (`self.Take Damage Sound Effects`)) (`self.K2_GetActorLocation`) (struct) 1.0 (`KismetMathLibrary.RandomFloatInRange` 0.8 1.2) 0.0 null null null null)
  (`NiagaraFunctionLibrary.SpawnSystemAtLocation` (`self.Take Damage System`) Normal (`KismetMathLibrary.MakeRotFromX` Location))
  (`self.OnTakeDamage`))

(event `/Game/EZ/Blueprints/DamageSystem/BPI_Damageable.Die`
  ; Die
  (`GameplayStatics.PlaySoundAtLocation` (`KismetArrayLibrary.Array_Random` (`self.Death Sound Effects`)) (`self.K2_GetActorLocation`) (struct) 0.4 (`KismetMathLibrary.RandomFloatInRange` 0.8 1.2) 0.0 null null null null)
  (`NiagaraFunctionLibrary.SpawnSystemAtLocation` "/Game/EZ/FX/FX_Explosion.FX_Explosion" (`SceneComponent.K2_GetComponentLocation` (`self.PaperFlipbook`)))
  (`|SpawnActorFromClass` "/Game/EZ/Sprites/Enemies/Alien_Ship/Pieces/Alien_Explosion.Alien_Explosion_C" (`SceneComponent.K2_GetComponentToWorld` (`self.PaperFlipbook`)) "AlwaysSpawn" "MultiplyWithRoot" null null)
  (`self.K2_DestroyActor`))

(event `self.PaperFlipbook.OnFinishedPlaying`
  ; On Animation Finished
  (`self.InitializeAnimations`))

(fn `Ground Actor`
  (bind (_returnvalue_x _returnvalue_y _returnvalue_z) (`KismetMathLibrary.BreakVector` (`self.K2_GetActorLocation`)))
  (bind _outhit (`KismetSystemLibrary.LineTraceSingle` (+ (`self.K2_GetActorLocation`) (0.0 0.0 25.0)) (+ (`self.K2_GetActorLocation`) (0.0 0.0 -150.0)) "TraceTypeQuery1"))
  (bind (_bblockinghit _binitialoverlap _time _distance _location _impactpoint) (`GameplayStatics.BreakHitResult` _outhit))
  (if (< (.z _impactpoint) _returnvalue_z)
    (`self.K2_SetActorLocation` (`KismetMathLibrary.MakeVector` _returnvalue_x _returnvalue_y (+ (`self.Ground Offset`) (.z _impactpoint))))))

(fn `InitializeAnimations`
  (`KismetSystemLibrary.PrintString` (`KismetStringLibrary.Concat_StrStr` "Initialize anims: " (`KismetSystemLibrary.GetDisplayName` self)))
  (`PaperFlipbookComponent.SetFlipbook` (`self.PaperFlipbook`) (`self.Idle Animation`))
  (`PaperFlipbookComponent.SetLooping` (`self.PaperFlipbook`) true)
  (`PaperFlipbookComponent.Play` (`self.PaperFlipbook`)))

(fn `LookAtLocation`
  (params (Location :type "Vector Structure"))
  (`self.K2_SetActorRotation` (`KismetMathLibrary.FindLookAtRotation` (`self.K2_GetActorLocation`) Location)))

(fn `MoveTowardsLocation`
  (params (targetLocation :type "Vector Structure") (DeltaTime :type "Float (double-precision)"))
  (`self.AddMovementInput` (- (`local.targetLocation`) (`self.K2_GetActorLocation`))))

(fn `Spawn Projectile`
  (bind _returnvalue_location (`KismetMathLibrary.BreakTransform` (`SceneComponent.K2_GetComponentToWorld` (`self.ProjectileSpawnPoint`))))
  (`PaperFlipbookComponent.Stop` (`self.PaperFlipbook`))
  (`PaperFlipbookComponent.SetFlipbook` (`self.PaperFlipbook`) (`self.Shoot Animation`))
  (`PaperFlipbookComponent.SetLooping` (`self.PaperFlipbook`) false)
  (`PaperFlipbookComponent.Play` (`self.PaperFlipbook`))
  (`|SpawnActorFromClass` (`self.Projectile`) (`SceneComponent.K2_GetComponentToWorld` (`self.ProjectileSpawnPoint`)) "AlwaysSpawn" "MultiplyWithRoot" null null)
  (`GameplayStatics.PlaySoundAtLocation` (`KismetArrayLibrary.Array_Random` (`self.Laser Sounds`)) _returnvalue_location (struct) 0.6 (`KismetMathLibrary.RandomFloatInRange` 0.8 1.2) 0.0 null null null null))

(fn `TryGetPlayerReference`
  (bind _returnvalue (`GameplayStatics.GetPlayerPawn` 0))
  (`/Engine/EditorBlueprintResources/StandardMacros.IsValid` _returnvalue
    (:`Is Valid`
      (set `self.PlayerReference` _returnvalue)
      (`KismetSystemLibrary.PrintString` "setting player ref"))
    (:`Is Not Valid`
      (`KismetSystemLibrary.PrintString` "No player ref"))))

(fn `UserConstructionScript`)