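; AI controller for the Goober enemy, with routines to detect and attack golf balls.
; SearchForTarget sphere-overlaps physics bodies within the pawn's detection range, optionally drawing a debug sphere, and stores the first golf ball found as CurrentTarget.
; Attack checks that target against attack range and, when its golf mode is inactive, launches it via SpitOutFromMonster from above the pawn with a pitch-randomized sound.
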(fn `Attack`
  (bind _returnvalue (`self.K2_GetActorLocation` (`self.K2_GetPawn`)))
  (bind _asbp_golf_ball (cast `/Game/Pants/Blueprints/BP_GolfBall` (`self.Current Target`)))
  (if (< (`KismetMathLibrary.Vector_Distance` _returnvalue (`self.K2_GetActorLocation` _asbp_golf_ball)) (`/Game/EZ/Blueprints/AI/BP_Enemy_Base.AttackRange` (`self.Enemy Pawn Reference`)))
    (if (not (`/Game/Pants/Blueprints/BP_GolfBall.bGolfModeActive` _asbp_golf_ball))
      (`/Game/Pants/Blueprints/BP_GolfBall.SpitOutFromMonster` _asbp_golf_ball (+ _returnvalue (0.0 0.0 60.0)) 800.0 1200.0 0.5 false (0.0 0.0 0.0) 20.0)
      (`KismetSystemLibrary.PrintString` "hit")
      (`GameplayStatics.PlaySoundAtLocation` "/Game/EZ/SFX/Bloop.Bloop" _returnvalue (struct) 0.7 (`KismetMathLibrary.RandomFloatInRange` 0.8 1.2) 0.0 null null null null))))

(fn `Search For Target`
  (bind _returnvalue (`self.K2_GetActorLocation` (`self.K2_GetPawn`)))
  (bind _detection_range (`/Game/EZ/Blueprints/AI/BP_Enemy_Base.Detection Range` (`self.Enemy Pawn Reference`)))
  ; Search For Target
  (if (`self.Debug`)
    (`KismetSystemLibrary.DrawDebugSphere` _returnvalue _detection_range 12 (struct :`R` 1.0 :`G` 0.409537 :`B` 0.952164 :`A` 1.0) 3.0 0.5))
  (bind _outactors (`KismetSystemLibrary.SphereOverlapActors` _returnvalue _detection_range (`|MakeArray` "ObjectTypeQuery4" :!type "EObjectTypeQuery Enum") "/Game/Pants/Blueprints/BP_GolfBall.BP_GolfBall_C"))
  (for _array_element _outactors
    (cast `/Game/Pants/Blueprints/BP_GolfBall` _array_element)
    (set `self.Current Target` _array_element)
    (break))
  (return))

(fn `UserConstructionScript`
  (`parent.UserConstructionScript`))