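; Loch Ness monster water hazard that catches a golf ball and spits it back out toward a target marker.
; A trigger overlap puts the ball in the hazard, then after a delay shows the sprite playing its throw flipbook.
; Tick, enabled only during recovery, watches for a specific flipbook frame to fire the spit once.
; The monster then idles, reverses its appear animation and hides; the construction script places trigger and target.
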(event `self.ReceiveBeginPlay`
  (`PaperFlipbookComponent.Stop` (`self.Sprite Flipbook`))
  (`SceneComponent.SetVisibility` (`self.Sprite Flipbook`) false false)
  (`self.SetActorTickEnabled` false))

(event `Start Animation Loop`
  (bind _sprite_flipbook (`self.Sprite Flipbook`))
  (set `self.reversed` false)
  (`PaperFlipbookComponent.SetFlipbook` _sprite_flipbook "/Game/EZ/Sprites/Enemies/LochNess/LochNess_Appear/LochNess_Appear.LochNess_Appear")
  (`PaperFlipbookComponent.SetLooping` _sprite_flipbook false)
  (`PaperFlipbookComponent.Play` _sprite_flipbook))

(event `self.Sprite Flipbook.OnFinishedPlaying`
  (bind _sprite_flipbook (`self.Sprite Flipbook`))
  (bind _sprite_flipbook_2 (`self.Sprite Flipbook`))
  (bind _sprite_flipbook_3 (`self.Sprite Flipbook`))
  (if (`self.reversed`)
    (`PaperFlipbookComponent.Stop` (`self.Sprite Flipbook`))
    (`SceneComponent.SetVisibility` (`self.Sprite Flipbook`) false false)
    (set `self.bRecoveringBall` false)
    (set `self.PendingGolfBall` null)
    (set `self.reversed` false)
    (`self.SetActorTickEnabled` false)
    (else
      (set `self.reversed` true)
      (`PaperFlipbookComponent.SetFlipbook` _sprite_flipbook_2 "/Game/EZ/Sprites/Enemies/LochNess/LochNess_Idle.LochNess_Idle")
      (`PaperFlipbookComponent.SetLooping` _sprite_flipbook_3 true)
      (`PaperFlipbookComponent.Play` _sprite_flipbook)
      (`KismetSystemLibrary.Delay` 1.0)
      (`PaperFlipbookComponent.SetFlipbook` _sprite_flipbook_2 "/Game/EZ/Sprites/Enemies/LochNess/LochNess_Appear/LochNess_Appear.LochNess_Appear")
      (`PaperFlipbookComponent.SetLooping` _sprite_flipbook_3 false)
      (`PaperFlipbookComponent.ReverseFromEnd` _sprite_flipbook))))

(event `self.ReceiveTick`
  (params (DeltaSeconds :type "Float (single-precision)"))
  (`self.TickAnimationFrame`))

(event `RecoverBall`
  (params (GolfBall :type "/Game/Pants/Blueprints/BP_GolfBall Object Reference"))
  (bind _sprite_flipbook (`self.Sprite Flipbook`))
  (set `self.PendingGolfBall` GolfBall)
  (set `self.bRecoveringBall` true)
  (set `self.bSpitFrameAlreadyFired` false)
  (set `self.reversed` false)
  (`SceneComponent.SetVisibility` _sprite_flipbook true false)
  (`PaperFlipbookComponent.SetFlipbook` _sprite_flipbook "/Game/EZ/Sprites/Enemies/LochNess/LochNess_Throw/LochNess_Throw.LochNess_Throw")
  (`PaperFlipbookComponent.SetLooping` _sprite_flipbook false)
  (`PaperFlipbookComponent.PlayFromStart` _sprite_flipbook)
  (`self.SetActorTickEnabled` true))

(event `self.WaterHazardTrigger.OnComponentBeginOverlap`
  (params (OverlappedComponent :type "PrimitiveComponent Object Reference") (OtherActor :type "Actor Object Reference") (OtherComp :type "PrimitiveComponent Object Reference") (OtherBodyIndex :type Integer) (bFromSweep :type Boolean) (SweepResult :type "HitResult Structure (by ref)"))
  (bind _asbp_golf_ball (cast `/Game/Pants/Blueprints/BP_GolfBall` OtherActor))
  (if (not (`self.bRecoveringBall`))
    (set `self.bRecoveringBall` true)
    (`GameplayStatics.PlaySoundAtLocation` (`self.WaterPloopSound`) (`self.K2_GetActorLocation` _asbp_golf_ball) (struct) 1.0 1.0 0.0 null null null null)
    (`/Game/Pants/Blueprints/BP_GolfBall.EnterWaterHazard` _asbp_golf_ball)
    (`KismetSystemLibrary.Delay` (`self.MonsterStartDelay`))
    (`self.RecoverBall` _asbp_golf_ball)))

(fn `SpitPendingBall`
  (bind _pendinggolfball (`self.PendingGolfBall`))
  (bind _spitpoint (`self.SpitPoint`))
  (`/Engine/EditorBlueprintResources/StandardMacros.IsValid` _pendinggolfball
    (:`Is Valid`
      (`GameplayStatics.PlaySoundAtLocation` "/Game/Pants/SFX/spit.spit" (`SceneComponent.K2_GetComponentLocation` _spitpoint) (struct) 1.0 1.0 0.0 null null null null)
      (`/Game/Pants/Blueprints/BP_GolfBall.SpitOutFromMonster` _pendinggolfball (`SceneComponent.K2_GetComponentLocation` _spitpoint) 1000.0 2000.0 1.0 true (`SceneComponent.K2_GetComponentLocation` (`self.TargetMarker`)) 20.0))))

(fn `TickAnimationFrame`
  (locals (`Frame Changed` :type Boolean))
  (set `self.Frame` (`PaperFlipbookComponent.GetPlaybackPositionInFrames` (`self.Sprite Flipbook`)))
  (bind _output_get (set `local.Frame Changed` (!= (`self.LastFrame`) (`self.Frame`))))
  (set `self.LastFrame` (`self.Frame`))
  ; This Only Fires if the frame changed this tick
  (if _output_get
    ;; Check For the correct Animation
    (if (== (`PaperFlipbookComponent.GetFlipbook` (`self.Sprite Flipbook`)) "/Game/EZ/Sprites/Enemies/LochNess/LochNess_Throw/LochNess_Throw.LochNess_Throw")
      ;; Pick the frame you want an event on
      (switch `int` (`self.Frame`)
        (:`5`
          (if (not (`self.bSpitFrameAlreadyFired`))
            (set `self.bSpitFrameAlreadyFired` true)
            (`self.SpitPendingBall`)))))))

(fn `UserConstructionScript`
  (`SceneComponent.K2_SetRelativeLocation` (`self.WaterHazardTrigger`) (`self.HazardOffset`) false false)
  (`BoxComponent.SetBoxExtent` (`self.WaterHazardTrigger`) (`self.HazardBoxExtent`) true)
  (`SceneComponent.K2_SetRelativeRotation` (`self.WaterHazardTrigger`) (`self.HazardBoxRotation`) false false)
  (`SceneComponent.K2_SetRelativeLocation` (`self.TargetMarker`) (`self.TargetOffset`) false false))