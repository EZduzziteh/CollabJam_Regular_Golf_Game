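; Alien abduction set piece that sucks a target ball up a beam and triggers the invasion.
; Tick lerps timed moves, ramps the beam's Z scale and applies a scaled pull force toward AbductionTargetPoint.
; The target's overlap destroys it, spawns an alien ship, switches music, gives the revolver with tutorial prompts and fires enemy spawners.
; It then kills distant enemies, maxes nearby enemies' detection ranges and destroys itself.
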(event `self.ReceiveTick`
  (params (DeltaSeconds :type "Float (single-precision)"))
  (bind _abductionbeamcontroller (`self.AbductionBeamController`))
  (bind _abductionbeamcontroller_2 (`self.AbductionBeamController`))
  (bind _abductionbeamcontroller_3 (`self.AbductionBeamController`))
  (bind _abductionbeamcontroller_4 (`self.AbductionBeamController`))
  (bind _ballmesh (`/Game/Pants/Blueprints/BP_GolfBall.BallMesh` (`self.Abduction Target`)))
  (bind _z (.z (`SceneComponent.RelativeScale3D` _abductionbeamcontroller_3)))
  (bind _z_2 (.z (`SceneComponent.RelativeScale3D` _abductionbeamcontroller)))
  ; Ramp Up Beam
  (`|ExecutionSequence`
    (:`then_0`
      (if (`self.moving`)
        (if (< (`self.moveTime`) (`self.Move Duration`))
          (set `self.moveTime` (+ (`self.moveTime`) DeltaSeconds))
          (`self.K2_SetActorLocation` (`KismetMathLibrary.VLerp` (`self.StartPosition`) (`self.TargetPosition`) (/ (`self.moveTime`) (`self.Move Duration`))))
          (else
            (`self.K2_SetActorLocation` (`KismetMathLibrary.VLerp` (`self.StartPosition`) (`self.TargetPosition`) 1.0))
            (set `self.moving` false)
            (`self.MoveCompleted`)))))
    (:`then_1`
      (if (`self.BeamActive`)
        (`|ExecutionSequence`
          (:`then_0`
            (if (not (`self.BeamFull`))
              (`SceneComponent.SetRelativeScale3D` _abductionbeamcontroller_3 (`KismetMathLibrary.MakeVector` (.x (`SceneComponent.RelativeScale3D` _abductionbeamcontroller_3)) (.y (`SceneComponent.RelativeScale3D` _abductionbeamcontroller_3)) (+ _z (* (`self.RampSpeed`) DeltaSeconds))))
              (if (> _z 1.0)
                (set `self.BeamFull` true)
                (`SceneComponent.SetRelativeScale3D` _abductionbeamcontroller_2 (`KismetMathLibrary.MakeVector` (.x (`SceneComponent.RelativeScale3D` _abductionbeamcontroller_2)) (.y (`SceneComponent.RelativeScale3D` _abductionbeamcontroller_2)) 1.0)))))
          (:`then_1`
            ; Handle Abduction Upwards Force
            (`/Engine/EditorBlueprintResources/StandardMacros.IsValid` (`self.Abduction Target`)
              (:`Is Valid`
                (`PrimitiveComponent.AddForce` _ballmesh (* (* (.z (`SceneComponent.RelativeScale3D` (`self.AbductionBeamController`))) (* DeltaSeconds (`self.Abduction Suck Force`))) (`KismetMathLibrary.Normal` (- (`SceneComponent.K2_GetComponentLocation` (`self.Abduction Target Point`)) (`SceneComponent.K2_GetComponentLocation` _ballmesh)))) "None" false)))))
        (elif (`self.BeamFull`)
          (`SceneComponent.SetRelativeScale3D` _abductionbeamcontroller (`KismetMathLibrary.MakeVector` (.x (`SceneComponent.RelativeScale3D` _abductionbeamcontroller)) (.y (`SceneComponent.RelativeScale3D` _abductionbeamcontroller)) (- _z_2 (* (`self.RampSpeed`) DeltaSeconds))))
          (if (<= _z_2 0.0)
            (set `self.BeamFull` false)
            (`SceneComponent.SetRelativeScale3D` _abductionbeamcontroller_4 (`KismetMathLibrary.MakeVector` (.x (`SceneComponent.RelativeScale3D` _abductionbeamcontroller_4)) (.y (`SceneComponent.RelativeScale3D` _abductionbeamcontroller_4)) 1.0))))))))

(event `Move to Location Over Seconds`
  (params (moveDuration :type "Float (double-precision)") (`Target Position` :type "Vector Structure"))
  (set `self.StartPosition` (`self.K2_GetActorLocation`))
  (set `self.TargetPosition` `Target Position`)
  (set `self.moveTime` 0.0)
  (set `self.Move Duration` moveDuration)
  (set `self.moving` true))

(event `Start Beam`
  (set `self.BeamActive` true))

(event `Set Abduction Target`
  (params (`new target` :type "/Game/Pants/Blueprints/BP_GolfBall Object Reference"))
  (set `self.Abduction Target` `new target`))

(event `self.Abduction Target Point.OnComponentBeginOverlap`
  (params (OverlappedComponent :type "PrimitiveComponent Object Reference") (OtherActor :type "Actor Object Reference") (OtherComp :type "PrimitiveComponent Object Reference") (OtherBodyIndex :type Integer) (bFromSweep :type Boolean) (SweepResult :type "HitResult Structure (by ref)"))
  (bind _returnvalue (`GameplayStatics.GetPlayerPawn` 0))
  (if (== (`self.Abduction Target`) OtherActor)
    (`self.K2_DestroyActor` OtherActor)
    (`|SpawnActorFromClass` "/Game/EZ/Blueprints/AI/BP_Enemy_Alien_Ship.BP_Enemy_Alien_Ship_C" (`KismetMathLibrary.MakeTransform` (`SceneComponent.K2_GetComponentLocation` (`self.Alien Ship Flipbook`))) "AlwaysSpawn" "MultiplyWithRoot" null null)
    (bind _returnvalue_2 (`GameplayStatics.GetActorOfClass` "/Game/EZ/Blueprints/BP_MusicManager.BP_MusicManager_C"))
    (`/Game/EZ/Blueprints/BP_MusicManager.Set Combat State` _returnvalue_2 "NewEnumerator2")
    (`GameplayStatics.PlaySoundAtLocation` "/Engine/EngineSounds/1kSineTonePing.1kSineTonePing" (`self.K2_GetActorLocation`) (struct) 1.0 1.0 0.0 null null null null)
    (bind _asbp_golf_shooter_character (cast `/Game/EZ/Blueprints/Player_Character/BP_Golf_Shooter_Character` (`GameplayStatics.GetPlayerPawn` 0)))
    (set `/Game/EZ/Blueprints/Player_Character/BP_Golf_Shooter_Character.Primary Weapon` "/Game/EZ/Blueprints/WeaponSystem/DataAssets/Weapon_Revolver.Weapon_Revolver" _asbp_golf_shooter_character)
    (`/Game/EZ/Blueprints/Player_Character/BP_Golf_Shooter_Character.Initialize Animations` _asbp_golf_shooter_character)
    (`|ExecutionSequence`
      (:`then_0`
        (bind _wbp_tutorial (`/Game/EZ/Blueprints/UI/WBP_Hud_EZ.WBP_Tutorial` (`/Game/EZ/Blueprints/Player_Character/BP_Golf_Shooter_Character.HudRef` _asbp_golf_shooter_character)))
        (`/Game/EZ/Blueprints/UI/WBP_Tutorial.Set All Unselected` _wbp_tutorial)
        (`Widget.SetVisibility` _wbp_tutorial "Visible")
        (`/Game/EZ/Blueprints/UI/WBP_Tutorial.Set Image Selected` _wbp_tutorial (`/Game/EZ/Blueprints/UI/WBP_Tutorial.Mouse_Left` _wbp_tutorial) true)
        (`/Game/EZ/Blueprints/UI/WBP_Tutorial.Set Image Selected` _wbp_tutorial (`/Game/EZ/Blueprints/UI/WBP_Tutorial.Mouse_Right` _wbp_tutorial) true))
      (:`then_1`
        (bind _returnvalue_3 (`GameplayStatics.GetActorOfClass` "/Game/EZ/Blueprints/BP_Game_Manager.BP_Game_Manager_C"))
        (set `/Game/EZ/Blueprints/BP_Game_Manager.IsInvasionTriggered` true _returnvalue_3))
      (:`then_2`
        (bind _outactors (`GameplayStatics.GetAllActorsOfClass` "/Game/Pants/Blueprints/BP_EnemySpawner.BP_EnemySpawner_C"))
        (for _array_element _outactors
          (`/Game/Pants/Blueprints/BP_EnemySpawner.SpawnEnemy` _array_element)
          (`self.K2_DestroyActor` _array_element)))
      (:`then_3`
        (bind _outactors_2 (`GameplayStatics.GetAllActorsOfClass` "/Game/EZ/Blueprints/AI/BP_Enemy_Base.BP_Enemy_Base_C"))
        (for _array_element_2 _outactors_2
          ; If enemies further than this, kill em
          (if (> (`KismetMathLibrary.Vector_Distance` (`self.K2_GetActorLocation` _array_element_2) (`self.K2_GetActorLocation` _returnvalue)) (`self.MaxKeepEnemyDistance`))
            (message `/Game/EZ/Blueprints/DamageSystem/BPI_Damageable.Die` _array_element_2)
            (else
              ; Otherwise make it so that enemies cant lose the player, get them assigned as a target.
              (set `/Game/EZ/Blueprints/AI/BP_Enemy_Base.LoseTargetRange` 1e+18 _array_element_2)
              (set `/Game/EZ/Blueprints/AI/BP_Enemy_Base.Detection Range` 1e+18 _array_element_2)
              (bind _asaic_enemy_base (cast `/Game/EZ/Blueprints/AI/AIC_Enemy_Base` (`AIBlueprintHelperLibrary.GetAIController` _returnvalue)))
              (`/Game/EZ/Blueprints/AI/AIC_Enemy_Base.SetCurrentTarget` _asaic_enemy_base _returnvalue)))))
      (:`then_4`
        (`self.K2_DestroyActor`)))))

(fn `UserConstructionScript`)