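; BP_Hole is a golf hole actor that detects when a golf ball lands in it.
; It caches the player pawn on BeginPlay and rotates every tick to face that pawn's location plus an offset.
; When a BP_GolfBall begins overlapping its sphere, it prints a hole message, plays a 2D sound and destroys the ball.
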(event `self.ReceiveBeginPlay`
  (set `self.PlayerReference` (`GameplayStatics.GetPlayerPawn` 0)))

(event `self.ReceiveTick`
  (params (DeltaSeconds :type "Float (single-precision)"))
  (`/Engine/EditorBlueprintResources/StandardMacros.IsValid` (`self.PlayerReference`)
    (:`Is Valid`
      (`self.K2_SetActorRotation` (`KismetMathLibrary.FindLookAtRotation` (`self.K2_GetActorLocation`) (+ (`self.K2_GetActorLocation` (`self.PlayerReference`)) (`self.Offset`)))))))

(event `self.Sphere.OnComponentBeginOverlap`
  (params (OverlappedComponent :type "PrimitiveComponent Object Reference") (OtherActor :type "Actor Object Reference") (OtherComp :type "PrimitiveComponent Object Reference") (OtherBodyIndex :type Integer) (bFromSweep :type Boolean) (SweepResult :type "HitResult Structure (by ref)"))
  (bind _asbp_golf_ball (cast `/Game/Pants/Blueprints/BP_GolfBall` OtherActor))
  (`KismetSystemLibrary.PrintString` "HOLE!")
  (`GameplayStatics.PlaySound2D` "/Engine/EditorSounds/GamePreview/EjectFromPlayer.EjectFromPlayer" 1.0 1.0 0.0 null null)
  (`self.K2_DestroyActor` _asbp_golf_ball))

(fn `UserConstructionScript`)