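; BP_Hole is a hole actor that reacts to a golf ball entering it and continually rotates to face the player.
; On sphere overlap it plays a sound, stops the BP_GolfBall, then either destroys it or, with AbductBall set, starts a guarded alien abduction.
; The abduction actor spawns above and behind the player, targets and moves to the ball, then starts its beam when the move completes.
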(event `self.ReceiveBeginPlay`
  (set `self.PlayerReference` (`GameplayStatics.GetPlayerPawn` 0)))

(event `self.ReceiveTick`
  (params (DeltaSeconds :type "Float (single-precision)"))
  (`/Engine/EditorBlueprintResources/StandardMacros.IsValid` (`self.PlayerReference`)
    (:`Is Valid`
      (`self.K2_SetActorRotation` (`KismetMathLibrary.FindLookAtRotation` (`self.K2_GetActorLocation`) (+ (`self.K2_GetActorLocation` (`self.PlayerReference`)) (`self.Offset`)))))))

(event `self.Sphere.OnComponentBeginOverlap`
  (params (OverlappedComponent :type "PrimitiveComponent Object Reference") (OtherActor :type "Actor Object Reference") (OtherComp :type "PrimitiveComponent Object Reference") (OtherBodyIndex :type Integer) (bFromSweep :type Boolean) (SweepResult :type "HitResult Structure (by ref)"))
  (bind _returnvalue (`GameplayStatics.GetPlayerPawn` 0))
  (bind _asbp_golf_ball (cast `/Game/Pants/Blueprints/BP_GolfBall` OtherActor))
  (`GameplayStatics.PlaySound2D` "/Engine/EditorSounds/GamePreview/EjectFromPlayer.EjectFromPlayer" 1.0 1.0 0.0 null null)
  (`/Game/Pants/Blueprints/BP_GolfBall.Stop Ball Moving` _asbp_golf_ball)
  (if (`self.abductBall`)
    (`self.AbductionTriggered`
      (:`then`)
      (:`else`
        (set `self.AbductionTriggered` true)
        (bind _returnvalue_2 (`|SpawnActorFromClass` "/Game/EZ/Blueprints/BP_Abduction_With-Alien.BP_Abduction_With-Alien_C" (`KismetMathLibrary.MakeTransform` (- (+ (`self.K2_GetActorLocation` _returnvalue) (0.0 0.0 200.0)) (* (`self.GetActorForwardVector` _returnvalue) 500.0))) "AlwaysSpawn" "MultiplyWithRoot" null null))
        (`/Game/EZ/Blueprints/BP_Abduction_With-Alien.Set Abduction Target` _returnvalue_2 _asbp_golf_ball)
        (bind _returnvalue_location (`KismetMathLibrary.BreakTransform` (`self.GetTransform` _asbp_golf_ball)))
        (`/Game/EZ/Blueprints/BP_Abduction_With-Alien.Move to Location Over Seconds` _returnvalue_2 2.0 _returnvalue_location)
        (add `/Game/EZ/Blueprints/BP_Abduction_With-Alien.MoveCompleted` _returnvalue_2 (delegate `CustomEvent`))))
    (else
      (`self.K2_DestroyActor` OtherActor))))

(event `CustomEvent`
  (`/Game/EZ/Blueprints/BP_Abduction_With-Alien.Start Beam` (stale `self.Sphere.OnComponentBeginOverlap` _returnvalue_2)))

(fn `UserConstructionScript`)