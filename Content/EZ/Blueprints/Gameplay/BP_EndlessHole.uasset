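; Golf hole flag for an endless mode, where one hole passes to another each time the ball sinks.
; BeginPlay caches all other holes and shows or hides itself from StartHidden; Tick turns it to face the player pawn.
; On overlap with the endless golf ball, it plays a sound, zeroes ball velocity, hides itself, shows a random other hole and hands that to the ball.
; Hiding toggles sphere collision, beacon and flipbook visibility.
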(event `self.ReceiveBeginPlay`
  (set `self.PlayerReference` (`GameplayStatics.GetPlayerPawn` 0))
  (bind _outactors (`GameplayStatics.GetAllActorsOfClass` "BP_EndlessHole_C"))
  (`KismetArrayLibrary.Array_RemoveItem` _outactors self)
  (set `self.EndlessFlagsArray` _outactors)
  (if (`self.bStartHidden`)
    (`self.HideFlag`)
    (else
      (`self.ShowFlag`))))

(event `self.ReceiveTick`
  (params (DeltaSeconds :type "Float (single-precision)"))
  (`/Engine/EditorBlueprintResources/StandardMacros.IsValid` (`self.PlayerReference`)
    (:`Is Valid`
      (`self.K2_SetActorRotation` (`KismetMathLibrary.FindLookAtRotation` (`self.K2_GetActorLocation`) (+ (`self.K2_GetActorLocation` (`self.PlayerReference`)) (`self.Offset`)))))))

(event `self.Sphere.OnComponentBeginOverlap`
  (params (OverlappedComponent :type "PrimitiveComponent Object Reference") (OtherActor :type "Actor Object Reference") (OtherComp :type "PrimitiveComponent Object Reference") (OtherBodyIndex :type Integer) (bFromSweep :type Boolean) (SweepResult :type "HitResult Structure (by ref)"))
  (bind _asbp_endless_golf_ball (cast `/Game/Pants/Blueprints/BP_EndlessGolfBall` OtherActor))
  (`GameplayStatics.PlaySound2D` "/Game/Pants/SFX/BallHole2.BallHole2" 1.0 1.0 0.0 null null)
  (bind _ballmesh (`/Game/Pants/Blueprints/BP_EndlessGolfBall.BallMesh` _asbp_endless_golf_ball))
  (`PrimitiveComponent.SetPhysicsLinearVelocity` _ballmesh (0.0 0.0 0.0) false "None")
  (`PrimitiveComponent.SetPhysicsAngularVelocityInDegrees` _ballmesh (0.0 0.0 0.0) false "None")
  (`self.HideFlag`)
  (bind _asbp_endless_hole (cast `/Game/EZ/Blueprints/Gameplay/BP_EndlessHole` (`|GetArrayItem` (`self.EndlessFlagsArray`) (`KismetMathLibrary.RandomIntegerInRange` 0 (- (`KismetArrayLibrary.Array_Length` (`self.EndlessFlagsArray`)) 1)))))
  (`self.ShowFlag` _asbp_endless_hole)
  (`/Game/Pants/Blueprints/BP_EndlessGolfBall.GrabNewFlag` _asbp_endless_golf_ball _asbp_endless_hole))

(fn `HideFlag`
  (set `self.bStartHidden` true)
  (`PrimitiveComponent.SetCollisionEnabled` (`self.Sphere`) "NoCollision")
  (`SceneComponent.SetVisibility` (`self.BP_Hole_Beacon`) false false)
  (`SceneComponent.SetVisibility` (`self.Flipbook`) false false))

(fn `ShowFlag`
  (set `self.bStartHidden` false)
  (`PrimitiveComponent.SetCollisionEnabled` (`self.Sphere`) "QueryOnly")
  (`SceneComponent.SetVisibility` (`self.BP_Hole_Beacon`) true false)
  (`SceneComponent.SetVisibility` (`self.Flipbook`) true false))

(fn `UserConstructionScript`)