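; Spawner that recreates the player's saved kill tally as tumbling killed-enemy actors, one for each kill.
; On BeginPlay it async-loads the "Default" save and copies the soldier, nurse, ship and Goober kill counts.
; A self-calling event with random delays spawns random enemy classes in a box around itself until all counts are used up.
; Each spawn gets random rotation, torque and force on its Cube.
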(event `self.ReceiveBeginPlay`
  (bind _savegame (`AsyncActionHandleSaveGame.AsyncLoadGameFromSlot` "Default")
    (:`Completed`
      (`|ExecutionSequence`
        (:`then_0`
          (bind _asbp_golf_shooter_save_game (cast `/Game/EZ/Blueprints/GameState/BP_GolfShooter_SaveGame` _savegame))
          (set `self.Ships to Spawn` (`/Game/EZ/Blueprints/GameState/BP_GolfShooter_SaveGame.ShipAliensKilled` _asbp_golf_shooter_save_game))
          (set `self.Soldiers To Spawn` (`/Game/EZ/Blueprints/GameState/BP_GolfShooter_SaveGame.SoldierAliensKilled` _asbp_golf_shooter_save_game))
          (set `self.Nurses to Spawn` (`/Game/EZ/Blueprints/GameState/BP_GolfShooter_SaveGame.SexyAliensKilled` _asbp_golf_shooter_save_game))
          (set `self.Goobers to Spawn` (`/Game/EZ/Blueprints/GameState/BP_GolfShooter_SaveGame.GoobersKilled` _asbp_golf_shooter_save_game)))
        (:`then_1`
          (`self.Spawn Killed Enemies`))))))

(event `Spawn Killed Enemies`
  (if (> (+ (`self.Soldiers To Spawn`) (`self.Nurses to Spawn`) (`self.Ships to Spawn`) (`self.Goobers to Spawn`)) 0)
    (`self.Spawn Random Killed Enemy`)
    (`KismetSystemLibrary.Delay` (`KismetMathLibrary.RandomFloatInRange` 0.2 0.7))
    (`self.Spawn Killed Enemies`)))

(fn `Spawn Random Killed Enemy`
  (locals (`Available Classes` :type "Array of /Game/EZ/Blueprints/KilledEnemies/BP_KilledEnemy Class Reference") (`Selected Class` :type "/Game/EZ/Blueprints/KilledEnemies/BP_KilledEnemy Class Reference"))
  (bind _outitem (`KismetArrayLibrary.Array_Random` (`local.Available Classes`)))
  (`|ExecutionSequence`
    (:`then_0`
      (if (> (`self.Soldiers To Spawn`) 0)
        (`KismetArrayLibrary.Array_Add` (`local.Available Classes`) "/Game/EZ/Blueprints/KilledEnemies/BP_KilledEnemy_Soldier.BP_KilledEnemy_Soldier_C")))
    (:`then_1`
      (if (> (`self.Nurses to Spawn`) 0)
        (`KismetArrayLibrary.Array_Add` (`local.Available Classes`) "/Game/EZ/Blueprints/KilledEnemies/BP_KilledEnemy_SexyNurse.BP_KilledEnemy_SexyNurse_C")))
    (:`then_2`
      (if (> (`self.Ships to Spawn`) 0)
        (`KismetArrayLibrary.Array_Add` (`local.Available Classes`) "/Game/EZ/Blueprints/KilledEnemies/BP_KilledEnemy_Ship.BP_KilledEnemy_Ship_C")))
    (:`then_3`
      (if (> (`self.Goobers to Spawn`) 0)
        (`KismetArrayLibrary.Array_Add` (`local.Available Classes`) "/Game/EZ/Blueprints/KilledEnemies/BP_KilledEnemy_Goober.BP_KilledEnemy_Goober_C")))
    (:`then_4`
      (set `local.Selected Class` _outitem)
      (bind _returnvalue (`|SpawnActorFromClass` _outitem (`KismetMathLibrary.MakeTransform` (`KismetMathLibrary.RandomPointInBoundingBox` (`self.K2_GetActorLocation`) (200.0 200.0 200.0)) (`KismetMathLibrary.RandomRotator` true)) "AlwaysSpawn" "MultiplyWithRoot" null null))
      (bind _cube (`/Game/EZ/Blueprints/KilledEnemies/BP_KilledEnemy.Cube` _returnvalue))
      (`PrimitiveComponent.AddTorqueInDegrees` _cube (* (`KismetMathLibrary.RandomUnitVector`) (`KismetMathLibrary.RandomFloatInRange` 25000.0 50000.0)) "None" true)
      (`PrimitiveComponent.AddForce` _cube (* (`KismetMathLibrary.RandomUnitVector`) (`KismetMathLibrary.RandomFloatInRange` 500.0 1500.0)) "None" true)
      (if (== (`local.Selected Class`) "/Game/EZ/Blueprints/KilledEnemies/BP_KilledEnemy_SexyNurse.BP_KilledEnemy_SexyNurse_C")
        (`/Engine/EditorBlueprintResources/StandardMacros.DecrementInt` (`self.Nurses to Spawn`))
        (elif (== (`local.Selected Class`) "/Game/EZ/Blueprints/KilledEnemies/BP_KilledEnemy_Ship.BP_KilledEnemy_Ship_C")
          (`/Engine/EditorBlueprintResources/StandardMacros.DecrementInt` (`self.Ships to Spawn`))
          (elif (== (`local.Selected Class`) "/Game/EZ/Blueprints/KilledEnemies/BP_KilledEnemy_Soldier.BP_KilledEnemy_Soldier_C")
            (`/Engine/EditorBlueprintResources/StandardMacros.DecrementInt` (`self.Soldiers To Spawn`))
            (elif (== (`local.Selected Class`) "/Game/EZ/Blueprints/KilledEnemies/BP_KilledEnemy_Goober.BP_KilledEnemy_Goober_C")
              (`/Engine/EditorBlueprintResources/StandardMacros.DecrementInt` (`self.Goobers to Spawn`)))))))))

(fn `UserConstructionScript`)