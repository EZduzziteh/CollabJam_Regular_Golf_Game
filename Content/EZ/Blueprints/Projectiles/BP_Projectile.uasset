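; Base projectile actor that damages what it hits and expires after a maximum lifetime.
; The construction script feeds Speed into the projectile movement's initial speed, and BeginPlay sets the lifespan.
; A bullet mesh hit calls TakeDamage through the BPI_Damageable interface, then spawns impact particles and a pitch-randomized sound before destroying the projectile, whether or not the target was damageable.
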(event `self.ReceiveBeginPlay`
  (`self.SetLifeSpan` (`self.Max Life Time`)))

(event `self.Bullet Mesh.OnComponentHit`
  (params (HitComponent :type "PrimitiveComponent Object Reference") (OtherActor :type "Actor Object Reference") (OtherComp :type "PrimitiveComponent Object Reference") (NormalImpulse :type "Vector Structure") (Hit :type "HitResult Structure (by ref)"))
  (bind (_bblockinghit _binitialoverlap _time _distance _location _impactpoint) (`GameplayStatics.BreakHitResult` Hit))
  (`|ExecutionSequence`
    (:`then_0`
      (bind _asbpi_damageable (cast `/Game/EZ/Blueprints/BPI_Damageable` OtherActor))
      (`/Game/EZ/Blueprints/BPI_Damageable.TakeDamage` _asbpi_damageable (`self.Damage`)))
    (:`then_1`
      (`NiagaraFunctionLibrary.SpawnSystemAtLocation` (`self.Hit Particles`) _impactpoint)
      (`GameplayStatics.SpawnSoundAtLocation` (`self.Hit Sound Effect`) _impactpoint (struct) 0.15 (`KismetMathLibrary.RandomFloatInRange` 0.8 1.2) 0.0 null null)
      (`self.K2_DestroyActor`))))

(fn `UserConstructionScript`
  (set `ProjectileMovementComponent.InitialSpeed` (`self.Speed`) (`self.ProjectileMovement`)))