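; Alien ship actor that takes damage and destroys itself when its health runs out.
; TakeDamage lowers current health, plays a hit sound, then fires the OnTakeDamage dispatcher.
; BeginPlay binds that dispatcher to CheckAlive, which calls Die at zero health or below to play a death sound and destroy the actor.
; Both sounds play at the ship's location with randomized pitch for variety.
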(event `self.ReceiveBeginPlay`
  (add `self.OnTakeDamage` (delegate `Check Alive`)))

(event `Check Alive`
  (if (<= (`self.CurrentHealth`) 0)
    (`self.Die`)))

(event `/Game/EZ/BPI_Damageable.TakeDamage`
  (params (amount :type Integer))
  (set `self.CurrentHealth` (- (`self.CurrentHealth`) amount))
  (`GameplayStatics.PlaySoundAtLocation` "/Engine/VREditor/Sounds/UI/Teleport_Committed.Teleport_Committed" (`self.K2_GetActorLocation`) (struct) 0.3 (`KismetMathLibrary.RandomFloatInRange` 0.8 1.2) 0.0 null null null null)
  (`self.OnTakeDamage`))

(event `/Game/EZ/BPI_Damageable.Die`
  (`GameplayStatics.PlaySoundAtLocation` "/Engine/VREditor/Sounds/VR_teleport.VR_teleport" (`self.K2_GetActorLocation`) (struct) 0.4 (`KismetMathLibrary.RandomFloatInRange` 0.8 1.2) 0.0 null null null null)
  (`self.K2_DestroyActor`))

(fn `UserConstructionScript`)