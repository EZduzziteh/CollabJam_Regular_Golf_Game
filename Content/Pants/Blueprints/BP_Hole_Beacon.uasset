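; Beacon actor, apparently marking a hole, that can be shown or hidden and gently bobs up and down.
; It records the shared root's relative location at BeginPlay and, each tick while bobbing is enabled, offsets its Z with a sine of game time using configurable speed, amplitude and phase.
; SetBeaconActive toggles visibility of the root and its children and activates or deactivates the beacon particles.
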(event `self.ReceiveBeginPlay`
  (set `self.BobBaseRelativeLocation` (`SceneComponent.RelativeLocation` (`self.SharedRoot`))))

(event `self.ReceiveTick`
  (params (DeltaSeconds :type "Float (single-precision)"))
  (`self.BobBeacon`))

(fn `BobBeacon`
  (if (`self.bBobEnabled`)
    (`SceneComponent.K2_SetRelativeLocation` (`self.SharedRoot`) (`KismetMathLibrary.MakeVector` (.x (`self.BobBaseRelativeLocation`)) (.y (`self.BobBaseRelativeLocation`)) (+ (.z (`self.BobBaseRelativeLocation`)) (* (`KismetMathLibrary.Sin` (+ (* (`self.BobSpeed`) (`KismetSystemLibrary.GetGameTimeInSeconds`)) (`self.BobPhaseOffset`))) (`self.BobAmplitude`)))) false false)))

(fn `SetBeaconActive`
  (params (bActive :type Boolean))
  (bind _beaconparticles (`self.BeaconParticles`))
  (if bActive
    (`SceneComponent.SetVisibility` (`self.SharedRoot`) true true)
    (`ActorComponent.Activate` _beaconparticles false)
    (else
      (`ActorComponent.Deactivate` _beaconparticles)
      (`SceneComponent.SetVisibility` (`self.SharedRoot`) false true))))

(fn `UserConstructionScript`)