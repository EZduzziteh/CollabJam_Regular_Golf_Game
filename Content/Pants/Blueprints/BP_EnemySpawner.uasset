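; Enemy spawner actor that creates weighted-random enemies at its own transform, driven by time, stroke count or both.
; In time mode, a looping timer calls SpawnEnemy while a second timer periodically shortens that interval down to a minimum, restarting the spawn timer.
; In stroke mode, stroke notifications accumulate and trigger a spawn at every multiple of the stroke interval.
; PickEnemyToSpawn rolls across entry weights plus a spawn-nothing weight.
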(event `self.ReceiveBeginPlay`
  (set `self.StrokeCount` 0)
  (if (`self.bSpawnByTime`)
    (`self.StartSpawner`)))

(event `NotifyStrokeEventChanged`
  (params (NewStrokeCount :type Integer))
  (bind _strokespawninterval (`self.StrokeSpawnInterval`))
  (bind _output_get (set `self.StrokeCount` (+ NewStrokeCount (`self.StrokeCount`))))
  (if (`self.bSpawnByStrokes`)
    (if (> _strokespawninterval 0)
      (if (== (mod _output_get _strokespawninterval) 0)
        (`self.SpawnEnemy`)))))

(fn `PickEnemyToSpawn`
  (returns (SelectedEnemyClass :type "/Game/EZ/Blueprints/AI/BP_Enemy_Base Class Reference") (bShouldSpawn :type Boolean))
  (locals (TotalWeight :type "Float (double-precision)") (RunningWeight :type "Float (double-precision)") (Roll :type "Float (double-precision)"))
  (bind _enemyspawnentries (`self.EnemySpawnEntries`))
  (bind _spawnnothingweight (`self.SpawnNothingWeight`))
  (set `local.TotalWeight` (`self.SpawnNothingWeight`))
  (for _array_element _enemyspawnentries
    (bind _output_get (set `local.TotalWeight` (+ (`.SpawnWeight_7_84AFE1BF40AB024D50332F95F20DB346` (break `/Game/Pants/Blueprints/ST_EnemySpawnEntry` _array_element)) (`local.TotalWeight`)))))
  (bind _output_get_2 (set `local.Roll` (`KismetMathLibrary.RandomFloatInRange` 0.0 _output_get)))
  (bind _returnvalue (< _output_get_2 _spawnnothingweight))
  (if _returnvalue
    (bind _returnvalue_2 (not _returnvalue))
    (return null _returnvalue_2)
    (else
      (set `local.RunningWeight` _spawnnothingweight)
      (for _array_element_2 _enemyspawnentries
        (bind (_enemyclass _spawnweight) (break `/Game/Pants/Blueprints/ST_EnemySpawnEntry` _array_element_2))
        (bind _output_get_3 (set `local.RunningWeight` (+ _spawnweight (`local.RunningWeight`))))
        (if (<= (`local.Roll`) _output_get_3)
          (return _enemyclass _returnvalue_2))))))

(fn `RampSpawnRate`
  (set `self.CurrentSpawnInterval` (`KismetMathLibrary.FClamp` (- (`self.CurrentSpawnInterval`) (`self.IntervalDecreaseAmount`)) (`self.MinSpawnInterval`) (`self.BaseSpawnInterval`)))
  (`KismetSystemLibrary.K2_ClearAndInvalidateTimerHandle` (`self.SpawnTimerHandle`))
  (bind _returnvalue (`KismetSystemLibrary.K2_SetTimer` null "SpawnEnemy" (`self.CurrentSpawnInterval`) true))
  (set `self.SpawnTimerHandle` _returnvalue))

(fn `SpawnEnemy`
  (bind (_selectedenemyclass _bshouldspawn) (`self.PickEnemyToSpawn`))
  (if _bshouldspawn
    (if (`KismetSystemLibrary.IsValidClass` _selectedenemyclass)
      (`|SpawnActorFromClass` _selectedenemyclass (`self.GetTransform`) "Undefined" "MultiplyWithRoot" null null)
      (else
        (`KismetSystemLibrary.PrintString` "Selected enemy class is null")))))

(fn `StartSpawner`
  (bind _output_get (set `self.CurrentSpawnInterval` (`self.BaseSpawnInterval`)))
  (bind _returnvalue (`KismetSystemLibrary.K2_SetTimer` null "SpawnEnemy" _output_get true))
  (set `self.SpawnTimerHandle` _returnvalue)
  (bind _returnvalue_2 (`KismetSystemLibrary.K2_SetTimer` null "RampSpawnRate" (`self.TimeRampInterval`) true))
  (set `self.RampTimerHandle` _returnvalue_2))

(fn `UserConstructionScript`)